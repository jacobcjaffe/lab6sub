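; BP_Character is a player character with gaze-based interaction and point-to-teleport movement, plus mouse look and sideways axis movement.
; Each tick, a camera line trace stores any BP_interact_interface actor as the interaction target and the hit point, at fixed height, as the teleport destination.
; Move/Interact messages that target, copying Score from a BP_blueCube, or otherwise teleports if the surface normal points sufficiently upward.
; BeginPlay adds the WB_UI widget.
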(event `self.ReceiveBeginPlay`
  (bind _returnvalue (`|CreateWidget` "/Game/Blueprints/WB_UI.WB_UI_C" (`GameplayStatics.GetPlayerController` 0)))
  (`UserWidget.AddToViewport` _returnvalue 0))

(event `InputAxis|moveLeft`
  (params (AxisValue :type "Float (single-precision)"))
  ;[1 1 1] Input
  (`self.AddMovementInput` (`self.GetActorRightVector`) AxisValue))

(event `self.ReceiveTick`
  (params (DeltaSeconds :type "Float (single-precision)"))
  (`self.GazeCheck`))

(event `InputAxis|mouseX`
  (params (AxisValue :type "Float (single-precision)"))
  ;[1 1 1] Input
  (`self.AddControllerYawInput` AxisValue))

(event `InputAxis|mouseY`
  (params (AxisValue :type "Float (single-precision)"))
  ;[1 1 1] Input
  (`self.AddControllerPitchInput` AxisValue))

(event `GazeCheck`
  (bind _camera (`self.Camera`))
  (bind _returnvalue (`SceneComponent.K2_GetComponentLocation` _camera))
  ;[1 1 1] Gaze check
  (bind _outhit (`KismetSystemLibrary.LineTraceSingle` :`Start` _returnvalue :`End` (+ _returnvalue (* (`SceneComponent.GetForwardVector` _camera) 2000)) :`TraceChannel` "TraceTypeQuery1" :`DrawDebugType` "ForOneFrame"))
  (`|ExecutionSequence`
    (:`then_0`
      (bind (_bblockinghit _binitialoverlap _time _distance _location _impactpoint _normal _impactnormal _physmat _hitactor) (`GameplayStatics.BreakHitResult` _outhit))
      (if (`KismetSystemLibrary.DoesImplementInterface` _hitactor "/Game/Blueprints/BP_interact_interface.BP_interact_interface_C")
        (bind _output_get (set `self.InteractingActor` _hitactor))
        (else
          (set `self.InteractingActor` null))))
    (:`then_1`
      (`KismetMathLibrary.Vector_Set` (`self.traceLoc`) (.x _location) (.y _location) 112.0))))

(event `InputAction|Move/Interact`
  (params (Key :type "Key Structure"))
  (bind _interactingactor (`self.InteractingActor`))
  (:`Pressed`
    (`/Engine/EditorBlueprintResources/StandardMacros.IsValid` _interactingactor
      (:`Is Valid`
        (message `/Game/Blueprints/BP_interact_interface.interact` _interactingactor)
        (bind _asbp_blue_cube (cast `/Game/Blueprints/BP_blueCube` (stale `GazeCheck` _output_get)))
        (set `self.score` (`/Game/Blueprints/BP_blueCube.score` _asbp_blue_cube)))
      (:`Is Not Valid`
        (if (>= (.z (`.Normal` (`GameplayStatics.BreakHitResult` (stale `GazeCheck` _outhit)))) 0.2)
          (`self.K2_TeleportTo` (`self.traceLoc`) (`self.K2_GetActorRotation`)))))))

(event `self.ReceiveActorBeginOverlap`
  (params (OtherActor :type "Actor Object Reference"))
  (if (`KismetSystemLibrary.DoesImplementInterface` OtherActor "/Game/Blueprints/NewInterface.NewInterface_C")
    _))

(fn `UserConstructionScript`)