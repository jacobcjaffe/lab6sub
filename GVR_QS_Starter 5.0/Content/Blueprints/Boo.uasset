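; Boo is a ghost-like enemy actor that creeps toward player 0 only while it has not been recently rendered.
; Each tick it checks render state, halting and playing the Blend timeline when seen, or reversing it and moving without sweep at MoveSpeed when unseen.
; The timeline drives the sphere material's Translucency parameter, and debug prints report the approach.
; Any actor overlap or the Kill event destroys it.
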(event `self.ReceiveBeginPlay`
  (bind _returnvalue (`PrimitiveComponent.CreateDynamicMaterialInstance` (`self.sphere`) 0 null "None"))
  (set `self.translucentMaterialInstance` _returnvalue))

(event `self.ReceiveTick`
  (params (DeltaSeconds :type "Float (single-precision)"))
  (bind _returnvalue (`self.K2_GetActorLocation`))
  (bind _returnvalue_2 (+ (* (* (`KismetMathLibrary.Normal` (- (`self.K2_GetActorLocation` (`GameplayStatics.GetPlayerPawn` 0)) _returnvalue)) DeltaSeconds) (`self.moveSpeed`)) _returnvalue))
  (`|ExecutionSequence`
    (:`then_0`
      (if (`self.WasRecentlyRendered` 0.0)
        (bind (_direction _blend) (`Timeline|blend` :!label _label)
          (:`Update`
            (bind _output_get (set `self.blend value` _blend))
            (`MeshComponent.SetScalarParameterValueOnMaterials` (`self.sphere`) "Translucency" _output_get)))
        (else
          (`|ExecutionSequence`
            (:`then_0`
              (goto _label :!via `Reverse`))
            (:`then_1`
              (`KismetSystemLibrary.PrintString` "Boo is coming..." true true (struct :`G` 0.66 :`B` 1.0 :`A` 1.0) 0.5 "1")
              (set `self.vecLox` _returnvalue_2)
              (`self.K2_SetActorLocation` _returnvalue_2))))))
    (:`then_1`
      (`KismetSystemLibrary.PrintString` (`KismetStringLibrary.Conv_Vector3fToString` (`self.vecLox`)) true true (struct :`R` 0.572693 :`B` 1.0 :`A` 1.0) 0.3 "3"))))

(event `self.ReceiveActorBeginOverlap`
  (params (OtherActor :type "Actor Object Reference"))
  (`ActorComponent.K2_DestroyComponent` (`self.sphere`))
  (`self.K2_DestroyActor`))

(event `/Game/Blueprints/NewInterface.kill`
  (`self.K2_DestroyActor`))

(fn `UserConstructionScript`)