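; Interactable door Blueprint that slides a Door component between two relative positions.
; On Interact, the Closed flag selects whether the DoorDriver timeline plays or reverses.
; Each timeline update lerps the door's relative location from DoorStart to DoorEnd by the Driver track.
; Closed is also toggled on every update tick of the timeline, rather than once when the motion finishes.
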(event `/Game/Blueprints/BP_interact_interface.interact`
  (if (`self.closed`)
    (bind (_direction _driver) (`Timeline|DoorDriver` :!label _label)
      (:`Update`
        (`SceneComponent.K2_SetRelativeLocation` (`self.door`) (`KismetMathLibrary.VLerp` (`self.DoorStart`) (`self.DoorEnd`) _driver) false false)
        (set `self.closed` (not (`self.closed`)))))
    (else
      (goto _label :!via `Reverse`))))

(fn `UserConstructionScript`)